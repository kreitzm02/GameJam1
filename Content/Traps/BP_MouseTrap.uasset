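; Mouse trap actor that snaps shut on an approach overlap, knocking back and damaging players.
; Tick lerps the roll of the trip, holding bar and hammer meshes over the snap length, then plays the snap sound.
; If the overlapper is on the player channel, a debug-drawn box query immediately launches player characters away, damages them and destroys the approach box, without waiting for the animation.
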(event EventBeginPlay)

(event Collision|EventActorBeginOverlap
  (params (OtherActor :type Actor%20Object%20Reference)))

(event EventTick
  (params (DeltaSeconds :type Float%20%28single-precision%29))
  (if (Variables|Default|GetStartSnapping)
    (Variables|Default|SetLerpEllapsedTime (+ (Variables|Default|GetLerpEllapsedTime) DeltaSeconds))
    (CallFunction|StaticMeshRotationLerp (Variables|Default|GetTrip) 8.0 (Variables|Default|GetSnapAnimationLength) (Variables|Default|GetLerpEllapsedTime))
    (CallFunction|StaticMeshRotationLerp (Variables|Default|GetHoldingBar) -185.0 (Variables|Default|GetSnapAnimationLength) (Variables|Default|GetLerpEllapsedTime))
    (CallFunction|StaticMeshRotationLerp (Variables|Default|GetHammer) 178.0 (Variables|Default|GetSnapAnimationLength) (Variables|Default|GetLerpEllapsedTime))
    (Math|Float|CompareFloat (/ (Variables|Default|GetLerpEllapsedTime) (Variables|Default|GetSnapAnimationLength)) 1.0
      (:>
        _)
      (:==
        _))
    (Variables|Default|SetStartSnapping false)
    (Audio|PlaySound2D "/Game/Traps/SFX_MouseTrap.SFX_MouseTrap" 1.0 1.0 0.2 0 0 false)))

(event EventOnApproachOverlap
  (params (OverlappedComponent :type Primitive%20Component%20Object%20Reference) (OtherActor :type Actor%20Object%20Reference) (OtherComp :type Primitive%20Component%20Object%20Reference) (OtherBodyIndex :type Integer) (bFromSweep :type Boolean) (SweepResult :type Hit%20Result%20Structure%20%28by%20ref%29))
  (bind _returnvalue (Transformation|GetActorLocation))
  (bind _snaphitsize (Variables|Default|GetSnapHitSize))
  (Variables|Default|SetStartSnapping true)
  (if (Utilities|Enum|Equal(Enum) (Collision|GetCollisionObjectType OtherComp) "ECC_GameTraceChannel1")
    (bind _outactors (Collision|BoxOverlapActors _returnvalue _snaphitsize (Utilities|Array|MakeArray "ObjectTypeQuery7") 0 :!class /Script/Engine.KismetSystemLibrary))
    (Rendering|Debug|DrawDebugBox _returnvalue _snaphitsize "(R=1.000000,G=0.000000,B=0.000000,A=1.000000)" "0, 0, 0" 4.0 1.0)
    (for _array_element _outactors
      (bind _ascharacter (Utilities|Casting|CastToCharacter _array_element))
      (if (Utilities|Enum|Equal(Enum) (Collision|GetCollisionObjectType (Variables|/Script/Engine.Character|GetCapsuleComponent _ascharacter)) "ECC_GameTraceChannel1")
        (Character|LaunchCharacter _ascharacter (* (Class|KismetMathLibrary|VectorNormalUnsafe (- (Transformation|GetActorLocation _ascharacter) (Transformation|GetActorLocation))) (Variables|Default|GetKnockbackStrenght)) true true)
        (bind _asgame_jam_1character (Utilities|Casting|CastToGameJam1Character _ascharacter))
        (Game|Damage|ApplyDamage _asgame_jam_1character 1.0 0 self)
        (Class|MouseTrap|DestroyApproachBox)))))

(fn ConstructionScript)

(fn StaticMeshRotationLerp
  (params (StaticMesh :type Static%20Mesh%20Component%20Object%20Reference) (TargetRotaion :type Float%20%28double-precision%29) (TimeSpan :type Float%20%28double-precision%29) (EllapsedTime :type Float%20%28double-precision%29))
  (Transformation|SetRelativeRotation StaticMesh (Math|Rotator|MakeRotator (Math|Float|Lerp 0.0 TargetRotaion (Math|Float|Clamp(Float) (/ EllapsedTime TimeSpan))) 0.0 0.0) false false))