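; BP_MineTrap is a proximity mine that explodes and knocks characters away when a component on the custom GameTraceChannel1 object channel triggers its approach overlap.
; It spawns a Niagara explosion, then runs a sphere overlap at the hit radius and launches characters whose capsules use that channel radially outward.
; The mine applies no damage and destroys itself inside the loop, so only after launching a character.
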(event EventBeginPlay)

(event Collision|EventActorBeginOverlap
  (params (OtherActor :type Actor%20Object%20Reference)))

(event EventTick
  (params (DeltaSeconds :type Float%20%28single-precision%29)))

(event EventOnApproachOverlap
  (params (OverlappedComponent :type Primitive%20Component%20Object%20Reference) (OtherActor :type Actor%20Object%20Reference) (OtherComp :type Primitive%20Component%20Object%20Reference) (OtherBodyIndex :type Integer) (bFromSweep :type Boolean) (SweepResult :type Hit%20Result%20Structure%20%28by%20ref%29))
  (if (Utilities|Enum|Equal(Enum) (Collision|GetCollisionObjectType OtherComp) "ECC_GameTraceChannel1")
    (Niagara|SpawnSystematLocation (Variables|Default|GetExplosionNiagara) (Transformation|GetActorLocation))
    (bind _outactors (Collision|SphereOverlapActors (Transformation|GetActorLocation) (Variables|Default|GetExplosionHitRadius) (Utilities|Array|MakeArray "ObjectTypeQuery7") 0))
    (for _array_element _outactors
      (bind _ascharacter (Utilities|Casting|CastToCharacter _array_element))
      (if (Utilities|Enum|Equal(Enum) (Collision|GetCollisionObjectType (Variables|/Script/Engine.Character|GetCapsuleComponent _ascharacter)) "ECC_GameTraceChannel1")
        (Character|LaunchCharacter _ascharacter (* (Class|KismetMathLibrary|VectorNormalUnsafe (- (Transformation|GetActorLocation _ascharacter) (Transformation|GetActorLocation))) (Variables|Default|GetKnockbackStrenght)) true true)
        (Actor|DestroyActor)))))

(fn ConstructionScript)