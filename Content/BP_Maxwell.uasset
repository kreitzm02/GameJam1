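; Maxwell easter-egg-style actor that, when the player enters its radius, mutes background music, plays OIIAOIIA audio and becomes a disco beam emitter.
; Tick runs timed stages: two spin phases, a pause, then revealing a sphere and gliding to the BP_MaxwellGoDiscoPoint location.
; It then periodically line-traces in random downward cone directions, spawning DiscoBallBeamBP at each hit's midpoint, scaled to span the distance.
; Debug drawing remains enabled for radius and traces.
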(event OnAudioFinished(OIIAOIIA)
  (Audio|Components|Audio|Play (Variables|Default|GetOIIAOIIA) 6.0))

(event OnComponentBeginOverlap(ActivationRadius)
  (params (OverlappedComponent :type Primitive%20Component%20Object%20Reference) (OtherActor :type Actor%20Object%20Reference) (OtherComp :type Primitive%20Component%20Object%20Reference) (OtherBodyIndex :type Integer) (bFromSweep :type Boolean) (SweepResult :type Hit%20Result%20Structure%20%28by%20ref%29))
  (Utilities|Casting|CastToGameJam1Character OtherActor)
  (Variables|Default|SetShouldActivate true)
  (Components|Activation|Activate (Variables|Default|GetOIIAOIIA) false)
  (Components|DestroyComponent (Variables|Default|GetActivationRadius)))

(event EventBeginPlay
  (bind _activationsphereradius (Variables|Default|GetActivationSphereRadius))
  (Rendering|SetVisibility (Variables|Default|GetSphere) false false)
  (bind _returnvalue (Actor|GetActorOfClass "/Game/BP_MaxwellGoDiscoPoint.BP_MaxwellGoDiscoPoint_C"))
  (Variables|Default|SetMaxwellDiscoPointLocation (Transformation|GetActorLocation _returnvalue))
  (Components|Sphere|SetSphereRadius (Variables|Default|GetActivationRadius) _activationsphereradius true)
  (Rendering|Debug|DrawDebugSphere (Transformation|GetActorLocation) _activationsphereradius 12 "(R=1.000000,G=0.000000,B=0.000000,A=1.000000)" 1e+01))

(event Collision|EventActorBeginOverlap
  (params (OtherActor :type Actor%20Object%20Reference)))

(event EventTick
  (params (DeltaSeconds :type Float%20%28single-precision%29))
  (if (Variables|Default|GetShouldActivate)
    (if (Variables|Default|GetIsActivated)
      (if (Variables|Default|GetIsMoving)
        (if (Variables|Default|GetIsMoving)
          (Transformation|SetActorLocation self (Math|Interpolation|VInterpTo (Transformation|GetActorLocation self) (Variables|Default|GetMaxwellDiscoPointLocation) DeltaSeconds 5.0) false false)
          (bind _output_get (Variables|Default|SetPassedTime (+ DeltaSeconds (Variables|Default|GetPassedTime))))
          (Math|Float|CompareFloat _output_get (Variables|Default|GetInterval)
            (:>
              (Variables|Default|SetIsMoving false)
              (Variables|Default|SetPassedTime 0.0)
              (Variables|Default|SetInterval 0.395)
              (Variables|Default|SetBeamFireEnabled true))))
        (elif (Variables|Default|GetBeamFireEnabled)
          (bind _output_get_2 (Variables|Default|SetPassedTime (+ DeltaSeconds (Variables|Default|GetPassedTime))))
          (Math|Float|CompareFloat _output_get_2 (Variables|Default|GetInterval)
            (:>
              (CallFunction|FireBeaminRndmDownDir)
              (Variables|Default|SetPassedTime 0.0)))))
      (else
        (CallFunction|ActivateMaxwell DeltaSeconds)))))

(fn ConstructionScript)

(fn FireBeaminDir
  (params (Direction :type Vector))
  (bind _returnvalue (Transformation|GetActorLocation))
  (bind (_outhit _returnvalue_2) (Collision|LineTraceByChannel (Transformation|GetActorLocation) (+ (* (Math|Vector|Normalize Direction) (Variables|Default|GetLineTraceLength)) (Transformation|GetActorLocation)) "TraceTypeQuery1" false (Utilities|Array|MakeArray self) "ForDuration"))
  (if _returnvalue_2
    (Game|SpawnActorfromClass (Variables|Default|GetDiscoBallBeamBP) (Math|Transform|MakeTransform (+ _returnvalue (/ (- (.Location (Collision|BreakHitResult _outhit)) _returnvalue) (Variables|Default|GetDivideByTwo))) (Math|Conversions|RotationFromXVector (Math|Vector|Normalize (- (.Location (Collision|BreakHitResult _outhit)) _returnvalue))) (Math|Vector|MakeVector 1.0 1.0 (/ (Math|Vector|VectorLength (- (+ _returnvalue (/ (- (.Location (Collision|BreakHitResult _outhit)) _returnvalue) (Variables|Default|GetDivideByTwo))) _returnvalue)) 25.0))) "Undefined" "MultiplyWithRoot" 0 0)))

(fn MakeRandomVectorDownwards
  (return (Math|Random|RandomUnitVectorinConeinDegrees "0.000000,0.000000,-1.000000" 85.0)))

(fn FireBeaminRndmDownDir
  (bind _downwardsvector (CallFunction|MakeRandomVectorDownwards))
  (CallFunction|FireBeaminDir _downwardsvector))

(fn RotateMaxwell
  (params (RotationSpeed :type Float%20%28double-precision%29))
  (Transformation|AddRelativeRotation (Variables|Default|Get_etkjdoiqwhuiorhvuier) (Math|Rotator|MakeRotator 0.0 0.0 RotationSpeed) false false))

(fn ActivateMaxwell
  (params (DeltaTime :type Float%20%28double-precision%29))
  (bind _outactors (Actor|GetAllActorsOfClass "/Script/GameJam1.GameManager"))
  (Class|GameManager|MuteBackgroundMusic _outactors)
  (if (Variables|Default|GetGoCompleteHam)
    (bind _output_get (Variables|Default|SetPassedTimeInActivation (+ DeltaTime (Variables|Default|GetPassedTimeInActivation))))
    (Math|Float|CompareFloat _output_get (Variables|Default|GetIntervalInActivation)
      (:>
        (Rendering|SetVisibility (Variables|Default|GetSphere) true false)
        (Variables|Default|SetIsActivated true)
        (Variables|Default|SetIsMoving true)))
    (else
      (bind _output_get_2 (Variables|Default|SetPassedTimeInActivation (+ DeltaTime (Variables|Default|GetPassedTimeInActivation))))
      (Math|Float|CompareFloat _output_get_2 (Variables|Default|GetIntervalInActivation)
        (:>
          (if (Variables|Default|GetSecondRotate)
            (CallFunction|RotateMaxwell 1e+01)
            (Math|Float|CompareFloat _output_get_2 (Variables|Default|GetBreakIntervalInActivation)
              (:>
                (Variables|Default|SetPassedTimeInActivation 0.0)
                (Variables|Default|SetGoCompleteHam true)
                (Variables|Default|SetIntervalInActivation 1.0)))
            (else
              (CallFunction|RotateMaxwell 4e+01)
              (Math|Float|CompareFloat _output_get_2 (Variables|Default|GetBreakIntervalInActivation)
                (:>
                  (Variables|Default|SetPassedTimeInActivation 0.0)
                  (Variables|Default|SetSecondRotate true)
                  (Variables|Default|SetIntervalInActivation 1.4)
                  (Variables|Default|SetBreakIntervalInActivation 3.3))))))))))