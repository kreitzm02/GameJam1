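; Short-lived disco ball beam actor that damages a game jam character caught in its capsule and expires after one second.
; It checks actors already overlapping on BeginPlay and any that begin overlapping later.
; Only characters whose capsule uses a custom collision object type and cast to GameJam1Character take damage.
; A hit destroys the beam's capsule rather than the actor, which stops further overlap hits.
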(event OnComponentBeginOverlap(Capsule)
  (params (OverlappedComponent :type Primitive%20Component%20Object%20Reference) (OtherActor :type Actor%20Object%20Reference) (OtherComp :type Primitive%20Component%20Object%20Reference) (OtherBodyIndex :type Integer) (bFromSweep :type Boolean) (SweepResult :type Hit%20Result%20Structure%20%28by%20ref%29))
  (bind _ascharacter (Utilities|Casting|CastToCharacter OtherActor))
  (if (Utilities|Enum|Equal(Enum) (Collision|GetCollisionObjectType (Variables|/Script/Engine.Character|GetCapsuleComponent _ascharacter)) "ECC_GameTraceChannel1")
    (bind _asgame_jam_1character (Utilities|Casting|CastToGameJam1Character _ascharacter))
    (Game|Damage|ApplyDamage _asgame_jam_1character 1.0 0 self)
    (Components|DestroyComponent (Variables|Default|GetCapsule))))

(event EventBeginPlay
  (Actor|SetLifeSpan 1.0)
  (for _array_element (Collision|GetOverlappingActors (Variables|Default|GetCapsule) 0 :!class /Script/Engine.PrimitiveComponent)
    (bind _ascharacter (Utilities|Casting|CastToCharacter _array_element))
    (if (Utilities|Enum|Equal(Enum) (Collision|GetCollisionObjectType (Variables|/Script/Engine.Character|GetCapsuleComponent _ascharacter)) "ECC_GameTraceChannel1")
      (bind _asgame_jam_1character (Utilities|Casting|CastToGameJam1Character _ascharacter))
      (Game|Damage|ApplyDamage _asgame_jam_1character 1.0 0 self)
      (Components|DestroyComponent (Variables|Default|GetCapsule)))))

(event Collision|EventActorBeginOverlap
  (params (OtherActor :type Actor%20Object%20Reference)))

(event EventTick
  (params (DeltaSeconds :type Float%20%28single-precision%29)))

(fn ConstructionScript)